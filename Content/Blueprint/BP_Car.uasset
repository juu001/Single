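; BP_Car is a self-driving vehicle that brakes for obstacles ahead of it.
; BeginPlay spawns its default controller and sets a random throttle capped by RandomSpeed.
; Each tick, a debug-drawn Visibility trace runs forward from the Arrow component, reacting only to skeletal mesh hits.
; Close hits apply handbrake, cut throttle and halve physics velocity; farther hits restore throttle, while no hit leaves inputs unchanged.
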(event Collision|EventActorBeginOverlap
  (params (OtherActor :type Actor%20Object%20Reference)))

(event EventBeginPlay
  (Utilities|FlowControl|Sequence
    (:then_0
      (Pawn|SpawnDefaultController))
    (:then_1
      (CallFunction|CarMoving))))

(event EventTick
  (params (DeltaSeconds :type Float%20%28single-precision%29))
  (CallFunction|CarLineTrace))

(fn ConstructionScript)

(fn CarMoving
  (bind _output_get (Variables|Default|SetThrottle (Math|Random|RandomFloatinRange 1e+01 (Variables|Default|GetRandomSpeed))))
  (Class|WheeledVehicleMovementComponent|SetThrottleInput (Variables|Default|GetVehicleMovement) _output_get))

(fn CarLineTrace
  (bind _arrow (Variables|Default|GetArrow))
  (bind _vehiclemovement (Variables|Default|GetVehicleMovement))
  (bind _vehiclemovement_2 (Variables|Default|GetVehicleMovement))
  (bind _returnvalue (Transformation|GetWorldLocation _arrow))
  (bind (_outhit _returnvalue_2) (Collision|LineTraceByChannel _returnvalue (+ _returnvalue (* (Math|Vector|GetForwardVector (Transformation|GetWorldRotation _arrow)) 1e+04)) "TraceTypeQuery1" false 0 "ForOneFrame"))
  (if _returnvalue_2
    (Utilities|Casting|CastToSkeletalMeshComponent (.HitComponent (Collision|BreakHitResult _outhit)))
    (if (< (.Distance (Collision|BreakHitResult _outhit)) 1e+03)
      (Class|WheeledVehicleMovementComponent|SetHandbrakeInput _vehiclemovement true)
      (Class|WheeledVehicleMovementComponent|SetThrottleInput _vehiclemovement 0.0)
      (bind _returnvalue_3 (Physics|GetPhysicsLinearVelocity (Variables|/Script/Engine.MovementComponent|GetUpdatedPrimitive (Variables|Default|GetVehicleMovement)) "Vechicle_Base"))
      (Class|PrimitiveComponent|SetAllPhysicsLinearVelocity (Variables|Character|GetMesh) (/ _returnvalue_3 2.0) false)
      (else
        (Class|WheeledVehicleMovementComponent|SetHandbrakeInput _vehiclemovement_2 false)
        (Class|WheeledVehicleMovementComponent|SetThrottleInput _vehiclemovement_2 (Variables|Default|GetThrottle))))))