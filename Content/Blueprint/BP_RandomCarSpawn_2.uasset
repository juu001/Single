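; Car spawner actor that keeps placing random cars at the center of its Boumd component.
; SpawnCar runs at BeginPlay, picking from CarClass and spawning at the bounds origin with a fixed rotation, adjusting for collisions but always spawning.
; When a component leaves Boumd, a two-second delay runs, then SpawnCar repeats if that component has the "car" tag.
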(event OnComponentEndOverlap(Boumd)
  (params (OverlappedComponent :type Primitive%20Component%20Object%20Reference) (OtherActor :type Actor%20Object%20Reference) (OtherComp :type Primitive%20Component%20Object%20Reference) (OtherBodyIndex :type Integer))
  (Utilities|FlowControl|Delay 2.0)
  (if (Components|ComponentHasTag OtherComp "car")
    (CallFunction|SpawnCar)))

(event Collision|EventActorBeginOverlap
  (params (OtherActor :type Actor%20Object%20Reference)))

(event EventTick
  (params (DeltaSeconds :type Float%20%28single-precision%29)))

(event EventBeginPlay
  (CallFunction|SpawnCar))

(fn ConstructionScript)

(fn SpawnCar
  (bind _carclass (Variables|Default|GetCarClass))
  (bind _outitem (Utilities|Array|Random _carclass))
  (if (Utilities|IsValidClass _outitem)
    (Game|SpawnActorfromClass _outitem (Math|Transform|MakeTransform (.Origin (Collision|GetComponentBounds (Variables|Default|GetBoumd))) "0.000000,180.000000,0.000000") "AdjustIfPossibleButAlwaysSpawn" 0 0)))